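; BP_AIGuyCharacter is an AI character that shows its current state and needs in an overhead-style widget bubble.
; A looping timer periodically pushes the AI state name and the first three need values, shown as Hunger, Fun and Energy, to the WBP_NeedsBubble widget.
; A helper formats each need as its name and floored value.
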(event Custom|Update%20UI%20values
  (bind _aswbp_needs_bubble (Utilities|Casting|CastToWBP_NeedsBubble (UserInterface|GetUserWidgetObject (Variables|Default|GetWidget))))
  (Default|UpdateCharacterValues _aswbp_needs_bubble (Class|AIGuyCharacter|GetAIStateName) (CallFunction|GetNeedValue) (CallFunction|GetNeedValue 1) (CallFunction|GetNeedValue 2)))

(event EventBeginPlay
  (Utilities|Time|SetTimerbyEvent (delegate Custom|Update%20UI%20values) 0.8 true))

(fn ConstructionScript)

(fn GetNeedValue
  (params (Index :type Integer))
  (bind _needs (Variables|Default|GetNeeds))
  (bind _output (Utilities|Array|Get(acopy) _needs Index))
  (return (Utilities|String|StringToName (Utilities|String|Append (.name _output) " = " (Utilities|String|ToString(Float) (Math|Conversions|ToFloat(Integer) (Math|Float|Floor (.value _output))))))))